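; BP_MyController is a controller Blueprint that drives the score and life HUD and handles the player's death.
; On BeginPlay it creates a WBP_UI widget and adds it to the viewport.
; Every Tick it pushes its Score and Life variables to the widget by polling, and destroys player 0's pawn when Life equals exactly zero.
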(event `self.ReceiveBeginPlay`
  (bind _returnvalue (`|CreateWidget` "/Game/WBP_UI.WBP_UI_C"))
  (bind _output_get (set `self.MyUI` _returnvalue))
  (`UserWidget.AddToViewport` _output_get 0))

(event `self.ReceiveTick`
  (params (DeltaSeconds :type "Float (single-precision)"))
  (bind _myui (`self.MyUI`))
  (bind _life (`self.Life`))
  (`/Game/WBP_UI.UpdateScore` _myui (`self.Score`))
  (`/Game/WBP_UI.UpdateLife` _myui _life)
  (if (== _life 0.0)
    (`self.K2_DestroyActor` (`GameplayStatics.GetPlayerPawn` 0))))

(fn `UserConstructionScript`)
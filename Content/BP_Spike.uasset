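; BP_Spike is a spike hazard that drains the player's life while the third-person character stands in its Box.
; Box begin and end overlap events toggle an IsHitting flag when the other actor is a BP_ThirdPersonCharacter.
; While the flag is set, Tick subtracts a small fixed amount from Life on player 0's BP_MyController, so the drain rate depends on frame rate.
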(event `self.ReceiveTick`
  (params (DeltaSeconds :type "Float (single-precision)"))
  (if (`self.IsHitting`)
    (bind _asbp_my_controller (cast `/Game/BP_MyController` (`GameplayStatics.GetPlayerController` 0)))
    (set `/Game/BP_MyController.Life` (- (`/Game/BP_MyController.Life` _asbp_my_controller) 0.001) _asbp_my_controller)))

(event `self.Box.OnComponentBeginOverlap`
  (params (OverlappedComponent :type "PrimitiveComponent Object Reference") (OtherActor :type "Actor Object Reference") (OtherComp :type "PrimitiveComponent Object Reference") (OtherBodyIndex :type Integer) (bFromSweep :type Boolean) (SweepResult :type "HitResult Structure (by ref)"))
  (cast `/Game/ThirdPerson/Blueprints/BP_ThirdPersonCharacter` OtherActor)
  (set `self.IsHitting` true))

(event `self.Box.OnComponentEndOverlap`
  (params (OverlappedComponent :type "PrimitiveComponent Object Reference") (OtherActor :type "Actor Object Reference") (OtherComp :type "PrimitiveComponent Object Reference") (OtherBodyIndex :type Integer))
  (cast `/Game/ThirdPerson/Blueprints/BP_ThirdPersonCharacter` OtherActor)
  (set `self.IsHitting` false))

(fn `UserConstructionScript`)